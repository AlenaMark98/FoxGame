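; BP_interact_object is an interactable actor that toggles a continuous spin around its local pitch axis.
; Each Begin call flips the Work flag and sets Speed, starting a fast looping timer when switched on.
; The timer applies local rotation scaled by Speed twice, so the step is Speed squared.
; Switching off zeroes Speed and leaves the timer running.
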(event `Begin`
  (bind _work (`self.work`))
  (if _work
    (set `self.work` false)
    (else
      (set `self.work` true)))
  (if _work
    (set `self.speed` 2.0)
    (`KismetSystemLibrary.K2_SetTimerDelegate` (delegate `start`) 0.01 true)
    (else
      (set `self.speed` 0.0))))

(event `start`
  (bind _speed (`self.speed`))
  (`self.K2_AddActorLocalRotation` (* (`KismetMathLibrary.MakeRotator` 0.0 _speed) _speed)))

(fn `UserConstructionScript`)