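; Interactable tap handle that toggles between two states each time it receives the Interaction event.
; A Work flag tracks the state and picks whether a timeline plays forward or reverses from the end, pitching the static mesh between zero and the Rotation value.
; Both toggles call Begin on a referenced InteractActor, leaving the linked effect to that actor.
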(event `/Game/Items/BP_Interact.Interaction`
  (bind _interact_actor (`self.Interact_Actor`))
  (if (`self.work`)
    (set `self.work` false)
    (`/Game/Interact/BP_interact_object.Begin` _interact_actor)
    (bind (_direction _newtrack_0) (`Timeline|Timeline_0` :!via `ReverseFromEnd` :!label _label)
      (:`Update`
        (`SceneComponent.K2_SetRelativeRotation` (`self.StaticMesh`) (`KismetMathLibrary.MakeRotator` 0.0 (`KismetMathLibrary.Lerp` 0.0 (`self.Rotation`) _newtrack_0)) false false)))
    (else
      (set `self.work` true)
      (`/Game/Interact/BP_interact_object.Begin` _interact_actor)
      (goto _label))))

(fn `UserConstructionScript`)