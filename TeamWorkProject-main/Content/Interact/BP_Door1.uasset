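; BP_Door1 is an interactable swinging door that toggles open and closed each time its Interaction event fires.
; On opening, it compares the mesh's rotation to a look-at rotation toward the character within 90 degrees to pick a positive or negative swing.
; A timeline lerps the mesh's relative yaw to that angle, and closing plays the same timeline in reverse from the end.
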(event `OpenDoor`
  (bind (_direction _newtrack_0) (`Timeline|Timeline_0` :!label _label)
    (:`Update`
      (`SceneComponent.K2_SetRelativeRotation` (`self.StaticMesh`) (`KismetMathLibrary.MakeRotator` 0.0 0.0 (`KismetMathLibrary.Lerp` 0.0 (`self.Rotation`) _newtrack_0)) false false))))

(event `CloseDoor`
  (goto _label :!via `ReverseFromEnd`))

(event `/Game/Items/BP_Interact.Interaction`
  (bind _staticmesh (`self.StaticMesh`))
  (if (`self.Door`)
    (set `self.Door` false)
    (`self.CloseDoor`)
    (else
      (set `self.Door` true)
      (if (== (`SceneComponent.K2_GetComponentRotation` _staticmesh) (`KismetMathLibrary.FindLookAtRotation` (`SceneComponent.K2_GetComponentLocation` _staticmesh) (`SceneComponent.K2_GetComponentLocation` (`Character.CapsuleComponent` (`self.Character`)))) :`ErrorTolerance` 90.0)
        (set `self.Rotation` 90.0)
        (else
          (set `self.Rotation` -90.0)))
      (`self.OpenDoor`))))

(fn `UserConstructionScript`)