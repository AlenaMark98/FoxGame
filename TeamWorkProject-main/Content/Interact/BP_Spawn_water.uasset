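; BP_Spawn_water is an interactable emitter that spawns Water actors while switched on.
; Its Begin event toggles the Work flag.
; While Work is true, Tick feeds a short Delay that throttles spawning of the Water object's class at the actor's location with zero rotation.
; The forward-vector offset is multiplied by zero, so it has no effect.
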(event `Begin`
  (if (`self.Work`)
    (set `self.work` false)
    (else
      (set `self.work` true))))

(event `self.ReceiveTick`
  (params (DeltaSeconds :type "Float (single-precision)"))
  (if (`self.work`)
    (`KismetSystemLibrary.Delay` 0.1)
    (`|SpawnActorFromClass` (`GameplayStatics.GetObjectClass` (`self.Water`)) (`KismetMathLibrary.MakeTransform` (+ (`self.K2_GetActorLocation`) (* (`self.GetActorForwardVector`) 0.0))) "Undefined" "OverrideRootScale" null null)))

(fn `UserConstructionScript`)