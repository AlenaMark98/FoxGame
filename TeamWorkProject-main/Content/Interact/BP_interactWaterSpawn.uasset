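; Interactable spawner actor, named for water, that spawns actors at its own location while a linked interactable is active.
; Each Tick it reads GetStats from the Link's BPInteractComponent.
; A true result runs a short Delay, which throttles the repeated spawning, then spawns an actor with zero rotation and unit scale.
; The forward-vector offset is zeroed, and the file does not show the spawned class.
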(event `self.ReceiveTick`
  (params (DeltaSeconds :type "Float (single-precision)"))
  (bind _work (`/Game/Interact/BP_InteractComponent.Get stats` (`/Game/Interact/BP_tap.BP_InteractComponent` (`self.link`))))
  (if _work
    (`KismetSystemLibrary.Delay` 0.1)
    (`|SpawnActorFromClass` "/Game/Interact/BP_Water.BP_Water_C" (`KismetMathLibrary.MakeTransform` (+ (`self.K2_GetActorLocation`) (* (`self.GetActorForwardVector`) 0.0))) "Undefined" "OverrideRootScale" null null)))

(fn `UserConstructionScript`)