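; BP_tap is an interactable tap whose static mesh rotates between two states on each interaction.
; The Interaction event flips the boolean state held in BPInteractComponent.
; A timeline plays forward when switching on and reverses from the end when switching off, lerping the mesh's relative pitch between zero and the Rotation variable.
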(event `/Game/Items/BP_Interact.Interaction`
  (bind _bp_interactcomponent (`self.BP_InteractComponent`))
  (bind _work (`/Game/Interact/BP_InteractComponent.Get stats` _bp_interactcomponent))
  (if _work
    (`/Game/Interact/BP_InteractComponent.Set stats` _bp_interactcomponent false)
    (bind (_direction _newtrack_0) (`Timeline|Timeline_0` :!via `ReverseFromEnd` :!label _label)
      (:`Update`
        (`SceneComponent.K2_SetRelativeRotation` (`self.StaticMesh`) (`KismetMathLibrary.MakeRotator` 0.0 (`KismetMathLibrary.Lerp` 0.0 (`self.Rotation`) _newtrack_0)) false false)))
    (else
      (`/Game/Interact/BP_InteractComponent.Set stats` _bp_interactcomponent true)
      (goto _label))))

(fn `UserConstructionScript`)